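; BP_Wall is a wall actor that drives a two-layer vertex-paint material with animated tiling on layer A.
; The construction script creates a dynamic instance of MI_VertexPaint on the Wall component and feeds it per-instance diffuse, ARM and normal textures plus tiling for both layers.
; Tick overrides layer A's tiling with a time-based sine lerp between 1 and MaxTiling.
; The Increasemaxtiling event raises that upper limit by one per call.
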(event `self.ReceiveTick`
  (params (DeltaSeconds :type "Float (single-precision)"))
  (`MaterialInstanceDynamic.SetScalarParameterValue` (`self.MID`) "Tilling_A" (`KismetMathLibrary.Lerp` 1.0 (`self.Max_tiling`) (+ (/ (`KismetMathLibrary.Sin` (* (`GameplayStatics.GetTimeSeconds`) (`self.Time_Speed`))) 2.0) 0.5))))

(event `Increase max tiling`
  (`/Engine/EditorBlueprintResources/StandardMacros.IncrementFloat` (`self.Max_tiling`)))

(fn `UserConstructionScript`
  (bind _returnvalue (`PrimitiveComponent.CreateDynamicMaterialInstance` (`self.Wall`) 0 "/Game/Materials/MI_VertexPaint.MI_VertexPaint" "None"))
  (bind _output_get (set `self.MID` _returnvalue))
  (`MaterialInstanceDynamic.SetTextureParameterValue` _output_get "Diffuse_A" (`self.Diffuse_A`))
  (`MaterialInstanceDynamic.SetTextureParameterValue` _output_get "Diffuse_B" (`self.Diffuse_B`))
  (`MaterialInstanceDynamic.SetTextureParameterValue` _output_get "ARM_A" (`self.ARM_A`))
  (`MaterialInstanceDynamic.SetTextureParameterValue` _output_get "ARM_B" (`self.ARM_B`))
  (`MaterialInstanceDynamic.SetTextureParameterValue` _output_get "Normal_A" (`self.Normal_A`))
  (`MaterialInstanceDynamic.SetTextureParameterValue` _output_get "Normal_B" (`self.Normal_B`))
  (`MaterialInstanceDynamic.SetScalarParameterValue` _output_get "Tilling_A" (`self.TillingA`))
  (`MaterialInstanceDynamic.SetScalarParameterValue` _output_get "Tilling_B" (`self.TillingB`)))